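; BP_Door is a locked door that the third-person player opens by spending a key.
; On actor overlap it casts to BP_ThirdPersonCharacter, decrements TotalKeys if any remain and plays the SwingDoorOpen timeline, otherwise printing a locked message.
; The timeline lerps the door mesh's yaw to swing it open, and any end overlap on OverlapBox reverses it to close the door.
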(event `self.ReceiveActorBeginOverlap`
  (params (OtherActor :type "Actor Object Reference"))
  (bind _asbp_third_person_character (cast `/Game/ThirdPerson/Blueprints/BP_ThirdPersonCharacter` OtherActor)) ; is it a player that ran into us?
  (if (> (`/Game/ThirdPerson/Blueprints/BP_ThirdPersonCharacter.TotalKeys` _asbp_third_person_character) 0)
    (`/Engine/EditorBlueprintResources/StandardMacros.DecrementInt` (`/Game/ThirdPerson/Blueprints/BP_ThirdPersonCharacter.TotalKeys` _asbp_third_person_character) ; subtact 1 from totalKeys
      (:`  `
        (`KismetSystemLibrary.PrintText` "Unlocking door!")
        (bind (_direction _newtrack_0) (`Timeline|Swing Door Open` :!label _label)
          (:`Update`
            (`SceneComponent.K2_SetRelativeRotation` (`self.SM_Bld_Door_01`) (`KismetMathLibrary.MakeRotator` 0.0 0.0 (`KismetMathLibrary.Lerp` 0.0 -90.0 _newtrack_0)) false false)))))
    (else
      (`KismetSystemLibrary.PrintText` "Locked!"))))

(event `self.OverlapBox.OnComponentEndOverlap`
  (params (OverlappedComponent :type "PrimitiveComponent Object Reference") (OtherActor :type "Actor Object Reference") (OtherComp :type "PrimitiveComponent Object Reference") (OtherBodyIndex :type Integer))
  (goto _label :!via `Reverse`))

(fn `UserConstructionScript`)