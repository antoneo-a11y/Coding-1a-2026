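; BP_Tree is a tree actor that simulates growth by changing the scale of its static mesh in three timed stages.
; BeginPlay chains randomized delays of a few seconds, each followed by a jump to a larger scale range, ending near full size.
; Each axis gets its own random value, so timing and proportions vary between instances.
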(event `self.ReceiveBeginPlay`
  (bind _returnvalue (`KismetMathLibrary.RandomFloatInRange` 0.7 0.9))
  (bind _returnvalue_2 (`KismetMathLibrary.RandomFloatInRange` 0.4 0.6))
  (bind _returnvalue_3 (`KismetMathLibrary.RandomFloatInRange` 0.9 1.1))
  (bind _returnvalue_4 (`KismetMathLibrary.RandomFloatInRange` 4.0 6.0))
  (`KismetSystemLibrary.Delay` _returnvalue_4)
  (`SceneComponent.SetRelativeScale3D` (`self.StaticMesh`) (`KismetMathLibrary.MakeVector` _returnvalue_2 _returnvalue_2 _returnvalue_2))
  (`KismetSystemLibrary.Delay` _returnvalue_4)
  (`SceneComponent.SetRelativeScale3D` (`self.StaticMesh`) (`KismetMathLibrary.MakeVector` _returnvalue _returnvalue _returnvalue))
  (`KismetSystemLibrary.Delay` _returnvalue_4)
  (`SceneComponent.SetRelativeScale3D` (`self.StaticMesh`) (`KismetMathLibrary.MakeVector` _returnvalue_3 _returnvalue_3 _returnvalue_3)))

(fn `UserConstructionScript`)